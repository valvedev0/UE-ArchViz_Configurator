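; First-person character for a furniture walkthrough, with axis movement, double-click move-to, a toggled flying drone mode, a pause menu and day/night level switching.
; Each tick a camera sphere trace finds "Usable" actors, toggling a HUD cursor and a floor decal that follows the mouse.
; Left click sends them a Use message.
; Collision overlaps with specific chair and sofa Blueprints show their edit buttons; right-mouse hold-to-move is defunct.
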(event `self.ReceiveBeginPlay`
  (bind _returnvalue (`GameplayStatics.GetPlayerController` 0))
  (`|ExecutionSequence`
    (:`then_0`
      ;[1 1 1] add default widget and show mouse cursor
      (bind _returnvalue_2 (`|CreateWidget` "/Game/Blueprints/widgets/Default.Default_C" _returnvalue))
      (bind _output_get (set `self.defaultWidget` _returnvalue_2))
      (`UserWidget.AddToViewport` _output_get 0)
      (set `PlayerController.bShowMouseCursor` true _returnvalue))
    (:`then_1`
      ;[1 1 1] HUD
      (bind _returnvalue_3 (`|CreateWidget` "/Game/Blueprints/UserIF/HUD_widget.HUD_widget_C" _returnvalue))
      (set `self.HUD` _returnvalue_3))))

(event `Key|RightMouseButton`
  (params (Key :type "Key Structure"))
  ;[0.9219 0.0557 0.1108] defunct
  ;;[1 1 1] Mouse and Touch Locomotion
  (:`Pressed`
    (bind _output_get (set `self.HeldTime` (+ (`self.HeldTime`) (`GameplayStatics.GetWorldDeltaSeconds`))))
    ;;[1 1 1] check if the actors are selected so dont move
    (if (>= _output_get (`self.HoldDuration`))
      (`/Engine/EditorBlueprintResources/StandardMacros.Gate` true :!via `Open` :!label _label
        (:`Exit`
          (`self.MoveToLocation` (`PlayerController.GetHitResultUnderCursorByChannel` (`GameplayStatics.GetPlayerController` 0) "TraceTypeQuery1" true))))))
  (:`Released`
    (set `self.HeldTime` 0.0)
    (goto _label :!via `Close`)))

(event `Key|Escape`
  (params (Key :type "Key Structure"))
  (bind _returnvalue (`GameplayStatics.GetPlayerController` 0))
  ;[1 1 1] menu widjet
  (:`Pressed`
    (bind _returnvalue_2 (`|CreateWidget` "/Game/Blueprints/UserIF/Menu_Widget.Menu_Widget_C" _returnvalue :!label _label_2))
    (`UserWidget.AddToViewport` _returnvalue_2 0)
    (`GameplayStatics.SetGamePaused` true)
    (`WidgetBlueprintLibrary.SetInputMode_UIOnlyEx` _returnvalue _returnvalue_2)
    (set `PlayerController.bShowMouseCursor` true _returnvalue)))

(event `Key|C`
  (params (Key :type "Key Structure"))
  ;[1 1 1] menu widjet
  (:`Pressed`
    (goto _label_2)))

(event `InputAxis|Moveforward`
  (params (AxisValue :type "Float (single-precision)"))
  ;[1 1 1] keyboard controller
  (`self.AddMovementInput` (`SceneComponent.GetForwardVector` (`self.Camera`)) AxisValue))

(event `InputAxis|Moveright`
  (params (AxisValue :type "Float (single-precision)"))
  ;[1 1 1] keyboard controller
  (`self.AddMovementInput` (`SceneComponent.GetRightVector` (`self.Camera`)) AxisValue))

(event `InputAxis|turnRate`
  (params (AxisValue :type "Float (single-precision)"))
  ;[1 1 1] keyboard controller
  (`self.AddControllerYawInput` AxisValue))

(event `InputAxis|LookUp`
  (params (AxisValue :type "Float (single-precision)"))
  ;[1 1 1] mouse control and touch control
  (`self.AddControllerPitchInput` AxisValue))

(event `self.ReceiveTick`
  (params (DeltaSeconds :type "Float (single-precision)"))
  (bind _camera (`self.Camera`))
  (bind _hud (`self.HUD`))
  (bind _returnvalue (`SceneComponent.K2_GetComponentLocation` _camera))
  (bind (_bblockinghit _binitialoverlap _time _distance _location _impactpoint _normal _impactnormal) (`GameplayStatics.BreakHitResult` (`PlayerController.GetHitResultUnderCursorByChannel` (`GameplayStatics.GetPlayerController` 0) "TraceTypeQuery1" true)))
  (`|ExecutionSequence`
    (:`then_0`
      ;[1 1 1] Tracing object
      (bind (_outhit _returnvalue_2) (`KismetSystemLibrary.SphereTraceSingleForObjects` _returnvalue (+ (* (`SceneComponent.GetForwardVector` _camera) 500) _returnvalue) 20.0 (`|MakeArray` "ObjectTypeQuery1" "ObjectTypeQuery2" :!type "EObjectTypeQuery Enum")))
      (if _returnvalue_2
        (if (`self.ActorHasTag` (`.HitActor` (`GameplayStatics.BreakHitResult` _outhit)) "Usable")
          (`/Game/Blueprints/UserIF/HUD_widget.Show mouse` _hud)
          (`SceneComponent.SetVisibility` (`self.Decal`) false false)
          (set `self.isSelectingActors` true)
          (else
            (`/Game/Blueprints/UserIF/HUD_widget.hide mouse` _hud :!label _label_3)
            (`SceneComponent.SetVisibility` (`self.Decal`) true false)
            (set `self.isSelectingActors` false)))
        (else
          (goto _label_3))))
    (:`then_1`
      ;[1 1 1] show decal in floor
      (if (not (`self.isSelectingActors`))
        (`SceneComponent.K2_SetWorldLocationAndRotation` (`self.Decal`) _location (`KismetMathLibrary.MakeRotationFromAxes` _impactnormal) false true)))))

(event `InputAxis|Turn`
  (params (AxisValue :type "Float (single-precision)"))
  ;[1 1 1] mouse control and touch control
  (`self.AddControllerYawInput` AxisValue))

(event `Key|LeftMouseButton`
  (params (Key :type "Key Structure"))
  (bind _camera (`self.Camera`))
  (bind _returnvalue (`SceneComponent.K2_GetComponentLocation` _camera))
  ;[1 1 1] Tracing object
  (:`Pressed`
    (`|ExecutionSequence`
      (:`then_0`
        (bind (_outhit _returnvalue_2) (`KismetSystemLibrary.SphereTraceSingleForObjects` _returnvalue (+ (* (`SceneComponent.GetForwardVector` _camera) 500) _returnvalue) 20.0 (`|MakeArray` "ObjectTypeQuery1" "ObjectTypeQuery2" :!type "EObjectTypeQuery Enum")))
        (if _returnvalue_2
          (bind (_bblockinghit _binitialoverlap _time _distance _location _impactpoint _normal _impactnormal _physmat _hitactor) (`GameplayStatics.BreakHitResult` _outhit))
          (if (`self.ActorHasTag` _hitactor "Usable")
            (message `/Game/Blueprints/MyactorINT.Use` _hitactor))))
      (:`then_1`
        ;[1 1 1] double tap locomotion
        (bind _result (`/Engine/EditorBlueprintResources/StandardMacros.IncrementInt` (`self.clickCount`))
          (:`  `
            (if (== _result 2)
              (`KismetSystemLibrary.PrintString` "doubleClick")
              (`self.MoveToLocation` (`PlayerController.GetHitResultUnderCursorByChannel` (`GameplayStatics.GetPlayerController` 0) "TraceTypeQuery1" true))))))))
  (:`Released`
    (`KismetSystemLibrary.RetriggerableDelay` 0.2)
    (set `self.clickCount` 0)))

(event `InputAxisKey|Gamepad_Special_Left_Y`
  (params (AxisValue :type "Float (single-precision)"))
  ;[1 1 1] mouse control and touch control
  (`self.AddControllerPitchInput` AxisValue))

(event `InputAxisKey|Gamepad_Special_Left_X`
  (params (AxisValue :type "Float (single-precision)"))
  ;[1 1 1] mouse control and touch control
  (`self.AddControllerYawInput` AxisValue))

(event `Key|H`
  (params (Key :type "Key Structure"))
  ;[1 1 1] drone mode
  (:`Pressed`
    (`/Engine/EditorBlueprintResources/StandardMacros.FlipFlop`
      (:`A`
        (`CharacterMovementComponent.SetMovementMode` (`self.CharacterMovement`) "MOVE_Flying" 0)
        (set `self.isFlying` true)
        (`KismetSystemLibrary.PrintString` "DroneMode Active" true true (struct :`G` 0.66 :`B` 1.0 :`A` 1.0) 10.0 "1"))
      (:`B`
        (`CharacterMovementComponent.SetMovementMode` (`self.CharacterMovement`) "MOVE_Walking" 0)
        (set `self.isFlying` false)
        (`KismetSystemLibrary.PrintString` "Walk Active" true true (struct :`G` 0.66 :`B` 1.0 :`A` 1.0) 10.0 "1")))))

(event `InputAxis|DroneModekey`
  (params (AxisValue :type "Float (single-precision)"))
  ;[1 1 1] drone mode
  (if (`self.isFlying`)
    (if (< AxisValue 0.0)
      (`self.AddMovementInput` (0.0 0.0 1.0) (* AxisValue (`self.flyrate`)))
      (else
        (`self.AddMovementInput` (0.0 0.0 1.0) (* AxisValue (`self.sinkrate`)))))))

(event `Key|N`
  (params (Key :type "Key Structure"))
  ;[1 1 1] day and night switch
  (:`Pressed`
    (`GameplayStatics.OpenLevel` "nightmap")
    (`KismetSystemLibrary.PrintString` "NightMode" true true (struct :`G` 0.66 :`B` 1.0 :`A` 1.0) 10.0)))

(event `Key|M`
  (params (Key :type "Key Structure"))
  ;[1 1 1] day and night switch
  (:`Pressed`
    (`GameplayStatics.OpenLevel` "newmap")
    (`KismetSystemLibrary.PrintString` "DayMode" true true (struct :`G` 0.66 :`B` 1.0 :`A` 1.0) 10.0)))

(event `self.Collison.OnComponentBeginOverlap`
  (params (OverlappedComponent :type "PrimitiveComponent Object Reference") (OtherActor :type "Actor Object Reference") (OtherComp :type "PrimitiveComponent Object Reference") (OtherBodyIndex :type Integer) (bFromSweep :type Boolean) (SweepResult :type "HitResult Structure (by ref)"))
  (bind _defaultwidget (`self.defaultWidget`))
  ;[1 1 1] start showinng buttons
  (`|ExecutionSequence`
    (:`then_0`
      (bind _assm_kreslo_04_blueprint (cast `/Game/Blueprints/SM_kreslo_04_Blueprint` OtherActor))
      (`KismetSystemLibrary.PrintString` "kursi")
      (set `self.kursi` _assm_kreslo_04_blueprint)
      (set `self.kursiAttached` true)
      (`Widget.SetVisibility` (`/Game/Blueprints/widgets/Default.Movebutton` _defaultwidget) "Visible")
      (`Widget.SetVisibility` (`/Game/Blueprints/widgets/Default.materialbutton` _defaultwidget) "Visible"))
    (:`then_1`
      (bind _assm_m_divan_05_blueprint_1 (cast `/Game/Blueprints/SM_M_Divan_05_Blueprint1` OtherActor))
      (set `self.Sofa01` _assm_m_divan_05_blueprint_1)
      (set `self.sofaAttached` true)
      (`Widget.SetVisibility` (`/Game/Blueprints/widgets/Default.ChangeObject` _defaultwidget) "Visible"))))

(event `self.Collison.OnComponentEndOverlap`
  (params (OverlappedComponent :type "PrimitiveComponent Object Reference") (OtherActor :type "Actor Object Reference") (OtherComp :type "PrimitiveComponent Object Reference") (OtherBodyIndex :type Integer))
  (bind _defaultwidget (`self.defaultWidget`))
  ;[1 1 1] stop showing buttons
  (`|ExecutionSequence`
    (:`then_0`
      (cast `/Game/Blueprints/SM_kreslo_04_Blueprint` OtherActor)
      (set `self.kursiAttached` false)
      (`Widget.SetVisibility` (`/Game/Blueprints/widgets/Default.materialbutton` _defaultwidget) "Hidden")
      (`Widget.SetVisibility` (`/Game/Blueprints/widgets/Default.Movebutton` _defaultwidget) "Hidden"))
    (:`then_1`
      (cast `/Game/Blueprints/SM_M_Divan_05_Blueprint1` OtherActor)
      (set `self.sofaAttached` false)
      (`Widget.SetVisibility` (`/Game/Blueprints/widgets/Default.ChangeObject` _defaultwidget) "Hidden"))))

(fn `dronemodee`
  (params (NewParam :type Boolean)))

(fn `MoveToLocation`
  (params (HitResult :type "HitResult Structure"))
  (bind (_bblockinghit _binitialoverlap _time _distance _location) (`GameplayStatics.BreakHitResult` HitResult))
  (bind _returnvalue (`GameplayStatics.GetPlayerController` 0))
  (if (>= (`KismetMathLibrary.VSize` (- _location (`self.K2_GetActorLocation` _returnvalue))) (`self.ClickDistance`))
    (`AIBlueprintHelperLibrary.SimpleMoveToLocation` _returnvalue _location)))

(fn `UserConstructionScript`)